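; BP_Bullet is a projectile actor that damages the player when fired by an enemy; player-fired hits only print a TODO.
; Initialize sets its direction, speed, owner side, lifetime and damage.
; Tick moves it in a straight line without sweep and counts down lifetime, but the expiry destroy check is unconnected.
; BulletCollision overlap calls TakeHit on BP_Player and destroys the bullet if it is an enemy projectile.
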(event OnComponentBeginOverlap(BulletCollision)
  (params (OverlappedComponent :type Primitive%20Component%20Object%20Reference) (OtherActor :type Actor%20Object%20Reference) (OtherComp :type Primitive%20Component%20Object%20Reference) (OtherBodyIndex :type Integer) (bFromSweep :type Boolean) (SweepResult :type Hit%20Result%20Structure%20%28by%20ref%29))
  (if (Variables|Default|GetIsEnemyProjectile)
    (bind _asbp_player (Utilities|Casting|CastToBP_Player OtherActor))
    (Default|TakeHit _asbp_player (Variables|Default|GetDamage))
    (Actor|DestroyActor)
    (else
      (Development|PrintString "TODO: Damage enemy"))))

(event EventBeginPlay)

(event Collision|EventActorBeginOverlap
  (params (OtherActor :type Actor%20Object%20Reference)))

(event EventTick
  (params (DeltaSeconds :type Float%20%28single-precision%29))
  (Transformation|SetActorLocation (+ (* (* (Variables|Default|GetTravelDirection) (Variables|Default|GetTravelSpeed)) (Utilities|Time|GetWorldDeltaSeconds)) (Transformation|GetActorLocation)) false false)
  (bind _output_get (Variables|Default|SetRemainingLifetime (- (Variables|Default|GetRemainingLifetime) (Utilities|Time|GetWorldDeltaSeconds)))))

(fn ConstructionScript)

(fn Initialize
  (params (Direction :type Vector) (Speed :type Float%20%28double-precision%29) (bIsEnemy :type Boolean) (Lifetime :type Float%20%28double-precision%29) (DamageValue :type Integer))
  (Variables|Default|SetTravelDirection (Math|Vector|Normalize Direction))
  (Variables|Default|SetTravelSpeed Speed)
  (Variables|Default|SetIsEnemyProjectile bIsEnemy)
  (Variables|Default|SetRemainingLifetime Lifetime)
  (Variables|Default|SetDamage DamageValue))