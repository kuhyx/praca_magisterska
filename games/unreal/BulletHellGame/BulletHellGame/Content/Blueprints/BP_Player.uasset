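; BP_Player is a player-controlled actor that moves on a bounded horizontal plane.
; BeginPlay registers the default Enhanced Input mapping context for the first player controller.
; Tick polls IA_Move, normalizes it, scales it by speed and delta time, then sets location without sweeping, with Z forced to zero.
; Both X and Y clamp between BoundsMin.X and BoundsMin.Y, so one vector supplies both limits.
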(event EventBeginPlay
  (Input|AddMappingContext (PlayerController|LocalPlayerSubsystems|GetEnhancedInputLocalPlayerSubsystem (Game|GetPlayerController 0)) "/Game/Input/IMC_Default.IMC_Default" 0 "(bIgnoreAllPressedKeysUntilRelease=True,bForceImmediately=False,bNotifyUserSettings=False)"))

(event Collision|EventActorBeginOverlap
  (params (OtherActor :type Actor%20Object%20Reference)))

(event EventTick
  (params (DeltaSeconds :type Float%20%28single-precision%29))
  (bind _returnvalue (Utilities|Time|GetWorldDeltaSeconds))
  (bind _returnvalue_2 (Transformation|GetActorLocation))
  (bind _returnvalue_3 (Input|EnhancedActionValues|GetIA_Move))
  (bind _movespeed (Variables|Default|GetMoveSpeed))
  (bind _boundsmin (Variables|Default|GetBoundsMin))
  (bind _boundsmin_2 (Variables|Default|GetBoundsMin))
  (bind _returnvalue_4 (Math|Vector|MakeVector (.x _returnvalue_3) (.y _returnvalue_3) 0.0))
  (bind _returnvalue_5 (* _returnvalue _movespeed))
  (bind _returnvalue_6 (Math|Vector|Normalize _returnvalue_4))
  (bind _returnvalue_7 (* _returnvalue_5 _returnvalue_6))
  (bind _returnvalue_8 (+ _returnvalue_2 _returnvalue_7))
  (Transformation|SetActorLocation (Math|Vector|MakeVector (Math|Float|Clamp(Float) (.x _returnvalue_8) (.x _boundsmin_2) (.y _boundsmin_2)) (Math|Float|Clamp(Float) (.y _returnvalue_8) (.x _boundsmin) (.y _boundsmin)) 0.0) false false))

(fn ConstructionScript)